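; BP_Projectile is a projectile that scores a point for the player when it hits an enemy.
; Each tick it moves its sphere components along world X at ForwardSpeed, scaled by delta time.
; On overlap, IsEnemy tests for a BP_Enemy class or subclass and increments BP_Player's Score on a match.
; The projectile destroys itself after scoring or on overlapping any non-enemy actor.
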(event EventBeginPlay)

(event EventTick
  (params (DeltaSeconds :type Float%20%28single-precision%29))
  (bind _forwardspeed (Variables|Default|GetForwardSpeed))
  (bind _sphere (Variables|Default|GetSphere))
  (bind _returnvalue (* DeltaSeconds _forwardspeed))
  (Transformation|AddWorldOffset (Variables|Default|GetSphere1) (Math|Vector|MakeVector _returnvalue 0.0 0.0) false false)
  (if (Utilities|IsValid _sphere)
    (Transformation|AddWorldOffset _sphere (Math|Vector|MakeVector _returnvalue 0.0 0.0) false false)))

(event Collision|EventActorBeginOverlap
  (params (OtherActor :type Actor%20Object%20Reference))
  (bind _newparam (CallFunction|IsEnemy OtherActor))
  (if _newparam
    (bind _asbp_player (Utilities|Casting|CastToBP_Player (Game|Player|GetPlayerPawn 0)))
    (Variables|/Game/InfiniteMatrix/Blueprints/BP_Player.BP_Player_C|SetScore _asbp_player (+ (Variables|/Game/InfiniteMatrix/Blueprints/BP_Player.BP_Player_C|GetScore _asbp_player) 1)))
  (Actor|DestroyActor))

(fn ConstructionScript)

(fn IsEnemy
  (params (Object :type Actor%20Object%20Reference))
  (return (Utilities|ClassIsChildOf (Utilities|GetClass Object) "/Game/InfiniteMatrix/Blueprints/BP_Enemy.BP_Enemy_C")))